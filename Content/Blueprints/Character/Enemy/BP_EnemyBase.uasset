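; BP_EnemyBase is the base enemy Blueprint, handling a spawn effect and an overhead HP bar widget.
; On BeginPlay a timeline animates the mesh's relative scale as a spawn effect, and the HP widget is cached as WBP_EnemyHP.
; UpdateHPProgressBar sets the current-to-max HP ratio and shows the bar, restarting a three-second timer that hides it again.
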(event `self.UpdateHPProgressBar`
  (`/Game/Blueprints/UI/ProgressBar/WBP_EnemyHP.UpdateHPPercent` (`self.WBP Enemy HP`) (/ (`self.GetCurrentHP`) (`self.GetMaxHP`)))
  ;[1 1 1] Visible And Hidden HP Bar
  (`Widget.SetVisibility` (`self.WBP Enemy HP`) "Visible")
  (`KismetSystemLibrary.K2_ClearAndInvalidateTimerHandle` (`self.HPBarHiddenTimer`))
  (bind _returnvalue (`KismetSystemLibrary.K2_SetTimerDelegate` (delegate `HPBarHidden_Event`) 3.0))
  (set `self.HPBarHiddenTimer` _returnvalue))

(event `HPBarHidden_Event`
  ;[1 1 1] Visible And Hidden HP Bar
  (`Widget.SetVisibility` (`self.WBP Enemy HP`) "Hidden"))

(event `self.ReceiveBeginPlay`
  (`|ExecutionSequence`
    (:`then_0`
      (bind (_direction _spawnedeffect) (`Timeline|Timeline`)
        (:`Update`
          (`SceneComponent.SetRelativeScale3D` (`self.Mesh`) (`KismetMathLibrary.MakeVector` _spawnedeffect _spawnedeffect _spawnedeffect)))))
    (:`then_1`
      (bind _aswbp_enemy_hp (cast `/Game/Blueprints/UI/ProgressBar/WBP_EnemyHP` (`WidgetComponent.GetUserWidgetObject` (`self.HPWidget`))))
      (set `self.WBP Enemy HP` _aswbp_enemy_hp))))

(fn `UserConstructionScript`)