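; BP_SaveMyselfCharacter is the player character, reacting to stage results and item placement confirmation.
; BeginPlay caches the player controller and binds the stage defeat, stage victory and item confirm delegates.
; Defeat and victory each play a barbarian animation and show a matching result widget.
; Item confirm turns the character toward the cursor hit point and plays a throw montage, whose notify triggers ActorSpawnComponent to confirm placement.
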(event `OnStageDefeatDelegate_Event`
  (`SkeletalMeshComponent.PlayAnimation` (`self.Mesh`) "/Game/Asset/KayKit/Characters/BarbarianAnimations/barbarian_Defeat.barbarian_Defeat" false)
  (bind _returnvalue (`|CreateWidget` "/Game/Blueprints/UI/StageStatus/WBP_DefeatWidget.WBP_DefeatWidget_C"))
  (`UserWidget.AddToViewport` _returnvalue 0))

(event `self.ReceiveBeginPlay`
  (`|ExecutionSequence`
    (:`then_0`
      (bind _asbp_save_myself_player_controller (cast `/Game/Blueprints/Player/BP_SaveMyselfPlayerController` (`GameplayStatics.GetPlayerController` 0)))
      (set `self.Save Myself Player Controller` _asbp_save_myself_player_controller))
    (:`then_1`
      (add `self.OnStageDefeatDelegate` (delegate `OnStageDefeatDelegate_Event`)))
    (:`then_2`
      (add `self.OnStageVictoryDelegate` (delegate `OnStageVictoryDelegate_Event`)))
    (:`then_3`
      (add `SaveMyselfPlayerController.ItemConfirmActionDelegate` (`self.Save Myself Player Controller`) (delegate `ItemConfirmActionDelegate_Event`)))))

(event `OnStageVictoryDelegate_Event`
  (`SkeletalMeshComponent.PlayAnimation` (`self.Mesh`) "/Game/Asset/KayKit/Characters/BarbarianAnimations/barbarian_Cheer.barbarian_Cheer" true)
  (bind _returnvalue (`|CreateWidget` "/Game/Blueprints/UI/StageStatus/WBP_VictoryWidget.WBP_VictoryWidget_C"))
  (`UserWidget.AddToViewport` _returnvalue 0))

(event `ItemConfirmActionDelegate_Event`
  (`self.K2_SetActorRelativeRotation` (`KismetMathLibrary.MakeRotator` 0.0 0.0 (`self.GetPlayerRotation`)))
  (`|PlayMontage` (`self.Mesh`) "/Game/Asset/KayKit/Characters/BarbarianAnimations/AM_barbarian_Throw.AM_barbarian_Throw"
    (:`OnNotifyBegin`
      (`ActorSpawnComponent.ConfirmPlacement` (`self.ActorSpawnComponent`)))))

(fn `GetPlayerRotation`
  (returns (Yaw :type "Float (single-precision)"))
  (return (.yaw (`KismetMathLibrary.FindLookAtRotation` (`self.K2_GetActorLocation`) (`.Location` (`GameplayStatics.BreakHitResult` (`PlayerController.GetHitResultUnderCursorByChannel` (`self.Save Myself Player Controller`) "TraceTypeQuery1" true)))))))

(fn `UserConstructionScript`)