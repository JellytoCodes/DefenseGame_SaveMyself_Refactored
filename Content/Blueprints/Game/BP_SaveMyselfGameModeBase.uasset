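; BP_SaveMyselfGameModeBase is the game mode that plays background music and stops it when the stage is won.
; On BeginPlay it sets and plays the BGM sound, then casts the first player's pawn to BP_SaveMyselfCharacter and caches it.
; It binds two events to that character's OnStageVictory delegate, both running the same logic that stops and destroys the BGM component.
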(event `self.ReceiveBeginPlay`
  (bind _bgm (`self.BGM`))
  (`AudioComponent.SetSound` _bgm (`self.Sound`))
  (`AudioComponent.Play` _bgm 0.0)
  (bind _asbp_save_myself_character (cast `/Game/Blueprints/Character/PlayerCharacter/BP_SaveMyselfCharacter` (`Controller.K2_GetPawn` (`GameplayStatics.GetPlayerController` 0))))
  (bind _output_get (set `self.BP Save Myself Character` _asbp_save_myself_character))
  (`/Engine/EditorBlueprintResources/StandardMacros.IsValid` _output_get
    (:`Is Valid`
      (add `SaveMyselfCharacter.OnStageVictoryDelegate` (`self.BP Save Myself Character`) (delegate `OnStageVictoryDelegate_Event_0`))
      (add `SaveMyselfCharacter.OnStageVictoryDelegate` (`self.BP Save Myself Character`) (delegate `OnStageVictoryDelegate_Event`)))))

(event `OnStageVictoryDelegate_Event_0`
  (bind _bgm (`self.BGM`))
  (`AudioComponent.Stop` _bgm :!label _label)
  (`ActorComponent.K2_DestroyComponent` _bgm))

(event `OnStageVictoryDelegate_Event`
  (goto _label))

(fn `UserConstructionScript`)